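; BPC_Inventory is an inventory component that, so far, only scans for pickable items around the player character.
; Every Tick runs a short multi-sphere trace on the Visibility channel, starting below player 0's actor location and extending along its forward vector, with per-frame debug drawing.
; Each hit actor is checked for the BPI_Pickable interface, but matches trigger no action and nothing is stored.
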(event EventBeginPlay)

(event EventTick
  (params (DeltaSeconds :type Float%20%28single-precision%29))
  (CallFunction|TraceItemtoPickUp))

(fn TraceItemtoPickUp
  (bind _returnvalue (Game|GetPlayerCharacter 0))
  (bind _returnvalue_2 (Transformation|GetActorLocation _returnvalue))
  (bind _returnvalue_3 (- _returnvalue_2 "0.000000,0.000000,60.000000"))
  (bind _outhits (Collision|MultiSphereTraceByChannel _returnvalue_3 (+ _returnvalue_3 (* (Transformation|GetActorForwardVector _returnvalue) 1e+01)) 5e+01 "TraceTypeQuery1" false 0 "ForOneFrame"))
  (for _array_element _outhits
    (if (Utilities|DoesObjectImplementInterface (.HitActor (Collision|BreakHitResult _array_element)) "/Game/Blueprints/Items/_Interfaces/BPI_Pickable.BPI_Pickable_C")
      _)))