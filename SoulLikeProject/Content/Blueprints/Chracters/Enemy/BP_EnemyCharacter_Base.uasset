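; Base enemy character Blueprint that handles spawn-in and death presentation with a material dissolve.
; On BeginPlay, a reversed timeline animates dissolve on mesh and equipped weapon while a random entry montage plays, if any exist.
; Death freezes animation, disables capsule collision and async-loads a Niagara effect tinted by the material's edge color.
; After loading, a timeline dissolves both meshes, then removes enemy widgets and destroys weapon and actor.
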(event EventBeginPlay
  (bind _entrymontagestoplay (Variables|Default|GetEntryMontagesToPlay))
  (Utilities|FlowControl|Sequence
    (:then_0
      (Components|Timeline|SetPlayRate (Variables|Default|GetEntryRestoreTimeLine) (/ 1.0 (Variables|Default|GetTotalEntryRestoreTime)))
      (bind _nomalizedfloattrack (Timeline|EntryRestoreTimeLine ReverseFromEnd)
        (:Update
          (CallFunction|HandleDissolveMaterial _nomalizedfloattrack _nomalizedfloattrack))))
    (:then_1
      (if (Utilities|Array|IsNotEmpty _entrymontagestoplay)
        (Animation|PlayAnimMontage (.OutItem (Utilities|Array|Random _entrymontagestoplay)) 1.0 "None")))))

(event EventOnEnemyDeath
  (params (DissolveNiagaraSystem :type Niagara%20System%20Soft%20Object%20Reference))
  (bind _mesh (Variables|Character|GetMesh))
  (Utilities|FlowControl|Sequence
    (:then_0
      ;[1 1 1] Pause Enemy Animation and Remove Collision
      (Variables|/Script/Engine.SkeletalMeshComponent|SetbPauseAnims (Variables|Character|GetMesh) true)
      (Collision|SetCollisionEnabled (Variables|Default|GetCapsuleComponent) "NoCollision"))
    (:then_1
      (bind _object (Utilities|AsyncLoadAsset DissolveNiagaraSystem)
        (:Completed
          (bind _asniagara_system (Utilities|Casting|CastToNiagaraSystem _object))
          (bind _returnvalue (Niagara|SpawnSystemAttached _asniagara_system (Variables|Character|GetMesh) "None" "0, 0, 0" "0, 0, 0" "KeepRelativeOffset" false))
          (bind _returnvalue_2 (Rendering|Material|CreateDynamicMaterialInstance _mesh 0 (Rendering|Material|GetMaterial _mesh 0) "None" :!class /Script/Engine.PrimitiveComponent))
          (bind _returnvalue_3 (Rendering|Material|GetVectorParameterValue _returnvalue_2 "DissolveEdgeColor" :!class /Script/Engine.MaterialInstanceDynamic))
          (Niagara|SetNiagaraVariable(LinearColor) _returnvalue "DissolveParticleColor" _returnvalue_3)
          (Components|Timeline|SetPlayRate (Variables|Default|GetDissolveTimeline) (/ 2.0 (Variables|Default|GetTotalDissolveTime)))
          (bind _nomalizedfloattrack (Timeline|DissolveTimeline PlayFromStart)
            (:Update
              (CallFunction|HandleDissolveMaterial _nomalizedfloattrack _nomalizedfloattrack))
            (:Finished
              (Class|EnemyUIComponent|RemoveEnemyDrawnWidgetsifAny (Variables|Default|GetEnemyUIComponent))
              (CallFunction|DestroyEnemy))))))))

(fn ConstructionScript)

(fn DestroyEnemy
  (bind _enemycombatcomponent (Variables|Default|GetEnemyCombatComponent))
  (bind _returnvalue (Class|PawnCombatComponent|GetCharacterCurrentEquippedWeapon _enemycombatcomponent))
  (Utilities|IsValid _returnvalue
    (:Is%20Valid
      (Actor|DestroyActor _returnvalue))
    (:Is%20Not%20Valid
      _))
  (Actor|DestroyActor))

(fn HandleDissolveMaterial
  (params (InputPin :type Float%20%28single-precision%29) (ParameterValue :type Float%20%28single-precision%29))
  (bind _enemycombatcomponent (Variables|Default|GetEnemyCombatComponent))
  (bind _returnvalue (Class|PawnCombatComponent|GetCharacterCurrentEquippedWeapon _enemycombatcomponent))
  (Rendering|Material|SetScalarParameterValueonMaterials (Variables|Character|GetMesh) "DissolveAmount" ParameterValue)
  (Utilities|IsValid _returnvalue
    (:Is%20Valid
      (Rendering|Material|SetScalarParameterValueonMaterials (Variables|/Script/SoulLikeProject.WarriorWeaponBase|GetWeaponMesh _returnvalue) "DissolveAmount" InputPin))))