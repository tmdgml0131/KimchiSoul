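; Hero character Blueprint that handles input for the pause menu and inventory screens.
; Both actions async-load their widget class on demand, then create it and add it to the viewport.
; Inventory input toggles the stored widget, switching between Game Only and Game And UI input modes and tracking open state with a boolean.
; The pause action only opens its screen, with no input mode change or removal here.
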(event Input|EnhancedActionEvents|EnhancedInputActionIA_PauseMenu
  (params (ActionValue :type Boolean) (ElapsedSeconds :type Float%20%28double-precision%29) (TriggeredSeconds :type Float%20%28double-precision%29) (InputAction :type Input%20Action%20Object%20Reference :default "/Game/Input/Input/Actions/IA_PauseMenu.IA_PauseMenu"))
  (:Started
    (bind _class (Utilities|AsyncLoadClassAsset "/Game/UI/Widgets/GameModeWidgets/WBP_PauseScreen.WBP_PauseScreen_C")
      (:Completed
        (bind _asuser_widget (Utilities|Casting|CastToUserWidgetClass _class))
        (bind _returnvalue (UserInterface|CreateWidget _asuser_widget))
        (UserInterface|Viewport|AddtoViewport _returnvalue 0)))))

(event Input|EnhancedActionEvents|EnhancedInputActionIA_OpenInventory
  (params (ActionValue :type Boolean) (ElapsedSeconds :type Float%20%28double-precision%29) (TriggeredSeconds :type Float%20%28double-precision%29) (InputAction :type Input%20Action%20Object%20Reference :default "/Game/Input/Input/Actions/IA_OpenInventory.IA_OpenInventory"))
  (:Started
    (if (Variables|Default|GetIsInventoryOpen)
      (Widget|RemovefromParent (Variables|Default|GetInventoryWIdget))
      (Class|WarriorFunctionLibrary|ToggleInputMode "GameOnly")
      (Variables|Default|SetIsInventoryOpen false)
      (else
        (bind _class (Utilities|AsyncLoadClassAsset "/Game/UI/Widgets/HeroWidgets/WBP_Inventory.WBP_Inventory_C")
          (:Completed
            (bind _asuser_widget (Utilities|Casting|CastToUserWidgetClass _class))
            (bind _returnvalue (UserInterface|CreateWidget _asuser_widget))
            (bind _output_get (Variables|Default|SetInventoryWIdget _returnvalue))
            (UserInterface|Viewport|AddtoViewport _output_get 0)
            (Class|WarriorFunctionLibrary|ToggleInputMode "GameAndUI")
            (Variables|Default|SetIsInventoryOpen true)))))))

(event EventBeginPlay)

(fn ConstructionScript)