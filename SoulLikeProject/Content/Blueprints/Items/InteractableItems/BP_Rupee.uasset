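; BP_Rupee is a money pickup actor whose mesh and value come from a row in the DT_Rupee data table.
; The construction script looks up the row named by its Money handle and sets the rupee's static mesh.
; When an actor tagged Player overlaps it, it casts to WarriorHeroCharacter, adds the row's Amount through HeroMoneyComponent, plays a pickup sound and destroys itself.
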(event Collision|EventActorBeginOverlap
  (params (OtherActor :type Actor%20Object%20Reference))
  (Class|WarriorFunctionLibrary|DoesActorHaveTag OtherActor "(TagName=\"Player\")"
    (:YES
      (bind _aswarrior_hero_character (Utilities|Casting|CastToWarriorHeroCharacter OtherActor))
      (bind _returnvalue (Utilities|GetDataTableRow "/Game/Blueprints/Items/_DataTable/DT_Rupee.DT_Rupee" (.rowname (Variables|Default|GetMoney)))
        (:then
          (Class|HeroMoneyComponent|AddMoney (Variables|/Script/SoulLikeProject.WarriorHeroCharacter|GetHeroMoneyComponent _aswarrior_hero_character) (.amount _returnvalue))
          (Audio|PlaySoundatLocation "/Game/Assets/Sounds/UI/A_UI_Select02.A_UI_Select02" (Transformation|GetActorLocation) "0, 0, 0" 1.0 1e+01 0.0 0 0 0 0)
          (Actor|DestroyActor))))))

(fn ConstructionScript
  (bind _returnvalue (Utilities|GetDataTableRow "/Game/Blueprints/Items/_DataTable/DT_Rupee.DT_Rupee" (.rowname (Variables|Default|GetMoney)))
    (:then
      (Components|StaticMesh|SetStaticMesh (Variables|Default|GetRupeeSM) (.staticmesh _returnvalue)))))