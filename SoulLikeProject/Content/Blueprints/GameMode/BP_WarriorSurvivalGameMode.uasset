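; Survival game mode Blueprint that shows on-screen wave announcements as the survival state changes.
; On BeginPlay it binds to the state-changed delegate and switches on the state to announce incoming, spawning and completed waves.
; Two helper functions create and add text widgets, one with a countdown driven by the wave wait time.
; On the last wave it also lengthens the enemy spawn delay and shows an extra banner after a pause.
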(event Custom|OnSurvivalGameModeStateChanged_Event
  (params (CurrentState :type EWarriorSurvivalGameModeState%20Enum :default "WaitSpawnNewWave"))
  (switch Utilities|FlowControl|Switch|SwitchonEWarriorSurvivalGameModeState CurrentState
    (:WaitSpawnNewWave
      (CallFunction|CreateWaveWidgetwithCountDown "New Wave Coming In!!" (Variables|Default|GetSpawnNewWaveWaitTime)))
    (:SpawningNewWave
      (CallFunction|CreateWaveWidgetNoCountDown (Utilities|Text|FormatText "Wave {CurrentWaveCount}" (Variables|Default|GetCurrentWaveCount)))
      (if (== (Variables|Default|GetCurrentWaveCount) (Variables|Default|GetTotalWavesToSpawn))
        (Variables|Default|SetSpawnEnemiesDelayTime 4.0)
        (Utilities|FlowControl|Delay 2.0)
        (CallFunction|CreateWaveWidgetNoCountDown "Last Wave!!")))
    (:WaveCompleted
      (CallFunction|CreateWaveWidgetNoCountDown (Utilities|Text|FormatText "Wave {CurrentWaveCount} Completed!" (Variables|Default|GetCurrentWaveCount))))))

(event EventBeginPlay
  (EventDispatchers|AssignOnSurvivalGameModeStateChanged (delegate Custom|OnSurvivalGameModeStateChanged_Event)))

(fn ConstructionScript)

(fn CreateWaveWidgetwithCountDown
  (params (TextContentToDisplay :type Text) (InTotalCountDownTime :type Float%20%28double-precision%29))
  (bind _returnvalue (UserInterface|CreateWidget "/Game/UI/Widgets/GameModeWidgets/WBP_WaveTextWithCountDown.WBP_WaveTextWithCountDown_C"))
  (UserInterface|Viewport|AddtoViewport _returnvalue 0)
  (Rendering|Components|TextRender|SetText (Variables|/Game/UI/Widgets/GameModeWidgets/WBP_WaveTextWithCountDown.WBP_WaveTextWithCountDown_C|GetTextBlock_WaveText _returnvalue) TextContentToDisplay)
  (Default|StartCountDown _returnvalue InTotalCountDownTime))

(fn CreateWaveWidgetNoCountDown
  (params (TextContentToDisplay :type Text))
  (bind _returnvalue (UserInterface|CreateWidget "/Game/UI/Widgets/GameModeWidgets/WBP_WaveTextNoCountDown.WBP_WaveTextNoCountDown_C"))
  (UserInterface|Viewport|AddtoViewport _returnvalue 0)
  (Rendering|Components|TextRender|SetText (Variables|/Game/UI/Widgets/GameModeWidgets/WBP_WaveTextNoCountDown.WBP_WaveTextNoCountDown_C|GetTextBlock_WaveText _returnvalue) TextContentToDisplay))